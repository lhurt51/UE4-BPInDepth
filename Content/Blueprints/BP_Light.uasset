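; BP_Light is an interactive spot light that the player can switch on and off with the F key while near it.
; A trigger volume enables player input on begin overlap and disables it on end overlap, toggling the HelpfulText prompt's visibility both times.
; The construction script applies the LightColor and VisSetting variables to set the spot light's colour and initial visibility.
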(event OnComponentBeginOverlap(Trigger)
  (params (OverlappedComponent :type Primitive%20Component%20Object%20Reference) (OtherActor :type Actor%20Object%20Reference) (OtherComp :type Primitive%20Component%20Object%20Reference) (OtherBodyIndex :type Integer) (bFromSweep :type Boolean) (SweepResult :type Hit%20Result%20Structure%20%28by%20ref%29))
  ;[0.2611 0.3895 1] When the tigger overlapps input is enabled and text is visible vic versa for end overlap
  (Input|EnableInput (Game|GetPlayerController 0))
  (Rendering|ToggleVisibility (Variables|Default|GetHelpfulText) false))

(event OnComponentEndOverlap(Trigger)
  (params (OverlappedComponent :type Primitive%20Component%20Object%20Reference) (OtherActor :type Actor%20Object%20Reference) (OtherComp :type Primitive%20Component%20Object%20Reference) (OtherBodyIndex :type Integer))
  ;[0.2611 0.3895 1] When the tigger overlapps input is enabled and text is visible vic versa for end overlap
  (Input|DisableInput (Game|GetPlayerController 0))
  (Rendering|ToggleVisibility (Variables|Default|GetHelpfulText) false))

(event EventBeginPlay)

(event Collision|EventActorBeginOverlap
  (params (OtherActor :type Actor%20Object%20Reference)))

(event EventTick
  (params (DeltaSeconds :type Float%20%28single-precision%29)))

(event Input|KeyboardEvents|F
  (params (Key :type Key%20Structure :default "AnyKey"))
  ;[1 0.1141 0.1041] Our f input toggles our spot lights visiblitilty
  (:Pressed
    (Rendering|ToggleVisibility (Variables|Default|GetSpotLight) false)))

(fn ConstructionScript
  (bind _spotlight (Variables|Default|GetSpotLight))
  (Rendering|Components|Light|SetLightColor _spotlight (Variables|Default|GetLightColor) true)
  (Rendering|SetVisibility _spotlight (Variables|Default|GetVisSetting) false))