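; BP_ExplosiveMat is an explosive hazard actor that shows objective text and blows up when its collision component is overlapped.
; Entering or leaving TriggerText toggles the GetTheObj message.
; Overlapping CollisionComp fires the Explosion effect, removes the mesh, toggles the objective text, shows OppsFailed, then destroys the actor after a short delay.
; The construction script sets initial text visibility and explosion auto-activation from variables, with no overlap filtering by actor.
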(event OnComponentBeginOverlap(CollisionComp)
  (params (OverlappedComponent :type Primitive%20Component%20Object%20Reference) (OtherActor :type Actor%20Object%20Reference) (OtherComp :type Primitive%20Component%20Object%20Reference) (OtherBodyIndex :type Integer) (bFromSweep :type Boolean) (SweepResult :type Hit%20Result%20Structure%20%28by%20ref%29))
  ;[1 0.1546 0.2044] Runs the explosion particle effects and destroys the actor when its done
  (Components|Activation|Activate (Variables|Default|GetExplosion) false)
  (Components|DestroyComponent (Variables|Default|GetStaticMeshComponent0))
  (Rendering|ToggleVisibility (Variables|Default|GetGetTheObj) false)
  (Rendering|SetVisibility (Variables|Default|GetOppsFailed) true false)
  (Utilities|FlowControl|Delay 1.25)
  (Actor|DestroyActor))

(event OnComponentBeginOverlap(TriggerText)
  (params (OverlappedComponent :type Primitive%20Component%20Object%20Reference) (OtherActor :type Actor%20Object%20Reference) (OtherComp :type Primitive%20Component%20Object%20Reference) (OtherBodyIndex :type Integer) (bFromSweep :type Boolean) (SweepResult :type Hit%20Result%20Structure%20%28by%20ref%29))
  ;[0.08993 1 0.9203] Toggles the objective message
  (Rendering|ToggleVisibility (Variables|Default|GetGetTheObj) false))

(event OnComponentEndOverlap(TriggerText)
  (params (OverlappedComponent :type Primitive%20Component%20Object%20Reference) (OtherActor :type Actor%20Object%20Reference) (OtherComp :type Primitive%20Component%20Object%20Reference) (OtherBodyIndex :type Integer))
  ;[0.08993 1 0.9203] Toggles the objective message
  (Rendering|ToggleVisibility (Variables|Default|GetGetTheObj) false))

(fn ConstructionScript
  (Rendering|SetVisibility (Variables|Default|GetGetTheObj) (Variables|Default|GetVisTextObj) false)
  (Rendering|SetVisibility (Variables|Default|GetOppsFailed) (Variables|Default|GetVisTextFailed) false)
  (Components|Activation|SetAutoActivate (Variables|Default|GetExplosion) (Variables|Default|GetVisExplosion)))